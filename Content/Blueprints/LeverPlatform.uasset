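; LeverPlatform is a moving platform Actor that slides between its start location and an EndPos, driven by an external Toggle event.
; It records its starting location on BeginPlay, and Toggle sets the direction of travel.
; Each Tick advances a clamped alpha forward or backward by Speed and lerps the position without sweep, so reversing mid-travel continues smoothly from the current point.
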(event `self.ReceiveBeginPlay`
  (set `self.StartPos` (`self.K2_GetActorLocation`)))

(event `self.ReceiveTick`
  (params (DeltaSeconds :type "Float (single-precision)"))
  (bind _output_get (set `self.LerpAlpha` (`KismetMathLibrary.FClamp` (+ (* (* DeltaSeconds (`self.Speed`)) (`KismetMathLibrary.SelectFloat` 1.0 -1.0 (`self.Toggled`))) (`self.LerpAlpha`)))))
  (`self.K2_SetActorLocation` (`KismetMathLibrary.VLerp` (`self.StartPos`) (`self.EndPos`) _output_get)))

(event `/Game/Blueprints/Toggleable.Toggle`
  (params (On :type Boolean))
  (set `self.Toggled` On))

(fn `UserConstructionScript`)