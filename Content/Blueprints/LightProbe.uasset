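; LightProbe counts how many lights reach the location of the actor that owns it.
; CountLights gathers all actors implementing LightInterface, asks each whether it Reaches the owner's location, and returns the number that do.
; Each light decides its own reach through the interface, and the probe does no work on BeginPlay or Tick.
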(fn `CountLights`
  (returns (NewParam :type Integer))
  (locals (Res :type Integer :default 0))
  (bind _outactors (`GameplayStatics.GetAllActorsWithInterface` "/Script/LightboyShadowgirl.LightInterface"))
  (for _array_element _outactors
    (bind _aslight_interface (cast `LightInterface` _array_element))
    (if (`LightInterface.Reaches` _aslight_interface (`Actor.K2_GetActorLocation` (`self.GetOwner`)))
      (`/Engine/EditorBlueprintResources/StandardMacros.IncrementInt` (`local.Res`))))
  (return (`local.Res`)))