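; PlayerSGChar is a 2D flipbook player character that restarts the current level when its LightProbe counts more than one light.
; Each tick it runs that light check and updates the sprite, showing run while moving on the ground and idle otherwise, including in the air.
; Move applies input along world X and flips the controller yaw to face the travel direction.
; BeginPlay sets a short jump hold time.
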(event `self.ReceiveBeginPlay`
  (set `self.JumpMaxHoldTime` 0.2))

(event `self.ReceiveTick`
  (params (DeltaSeconds :type "Float (single-precision)"))
  (`self.UpdateAnimation`)
  (if (> (`/Game/Blueprints/LightProbe.CountLights` (`self.LightProbe`)) 1)
    (bind _returnvalue (`GameplayStatics.GetCurrentLevelName` true))
    (`GameplayStatics.OpenLevel` (`KismetStringLibrary.Conv_StringToName` _returnvalue))))

(fn `Move`
  (params (NewParam :type "Float (double-precision)"))
  (`self.AddMovementInput` (1.0 0.0 0.0) NewParam)
  (`Controller.SetControlRotation` (`self.GetController`) (select `bool` (> NewParam 0.0) :`false` (`KismetMathLibrary.MakeRotator` 0.0 0.0 180.0) :`true` (`KismetMathLibrary.MakeRotator` 0.0))))

(fn `UpdateAnimation`
  (bind (_returnvalue_x _returnvalue_y _returnvalue_z) (`KismetMathLibrary.BreakVector` (`self.GetVelocity`)))
  (if (`NavMovementComponent.IsMovingOnGround` (`self.CharacterMovement`))
    (if (> (`KismetMathLibrary.VSize` (`self.GetVelocity`)) 0.0)
      (`PaperFlipbookComponent.SetFlipbook` (`self.Sprite`) "/Game/StarterContent/Sprites/Flipbooks/SG_Run.SG_Run")
      (else
        (`PaperFlipbookComponent.SetFlipbook` (`self.Sprite`) "/Game/StarterContent/Sprites/Flipbooks/SG_Idle.SG_Idle")))
    (elif (< _returnvalue_z -100.0)
      (`PaperFlipbookComponent.SetFlipbook` (`self.Sprite`) "/Game/StarterContent/Sprites/Flipbooks/SG_Idle.SG_Idle")
      (else
        (`PaperFlipbookComponent.SetFlipbook` (`self.Sprite`) "/Game/StarterContent/Sprites/Flipbooks/SG_Idle.SG_Idle")))))

(fn `UserConstructionScript`)