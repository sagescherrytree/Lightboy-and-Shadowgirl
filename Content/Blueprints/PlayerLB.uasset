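; LightBoy player Blueprint for a 2D side-scroller character who loses when outside the reach of every light.
; BeginPlay caches all LightInterface actors, and Tick queries them with the player's XZ position, calling Lose if none report reachable.
; Tick also picks run, idle, jump or fall flipbooks from movement, with a Delay pacing footsteps and flag-gated wind sounds.
; Move applies X-axis input and adjusts sprite X scale from the input.
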(event `self.ReceiveBeginPlay`
  (set `self.BaseScale` (`SceneComponent.RelativeScale3D` (`self.Sprite`)))
  (bind _outactors (`GameplayStatics.GetAllActorsWithInterface` "/Game/Blueprints/Lights/LightInterface.LightInterface_C"))
  (for _array_element _outactors
    (bind _aslight_interface (cast `/Game/Blueprints/Lights/LightInterface` _array_element))
    (`KismetArrayLibrary.Array_Add` (`self.Lights`) _aslight_interface)))

(event `self.ReceiveTick`
  (params (DeltaSeconds :type "Float (single-precision)"))
  (`self.UpdateAnimation`)
  (`self.LightCheck`)
  (`KismetSystemLibrary.Delay` 0.28)
  (`self.PlaySound`))

(fn `LightCheck`
  (for _array_element (`self.Lights`)
    (bind _isreachable (`/Game/Blueprints/Lights/LightInterface.isReachable` _array_element (`KismetMathLibrary.MakeVector2D` (.x (`self.K2_GetActorLocation`)) (.z (`self.K2_GetActorLocation`)))))
    (if _isreachable
      (return)))
  (`KismetSystemLibrary.PrintString` "LightBoy Dies :(")
  (`/Game/Blueprints/Lib.Lose`))

(fn `Move`
  (params (Amount :type "Float (double-precision)"))
  (`self.AddMovementInput` (1.0 0.0 0.0) Amount)
  (bind _result (`/Engine/EditorBlueprintResources/StandardMacros.NegateFloat` (* (.x (`self.BaseScale`)) Amount))
    (:`  `
      (`SceneComponent.SetRelativeScale3D` (`self.Sprite`) (`KismetMathLibrary.MakeVector` _result (.y (`self.BaseScale`)) (.z (`self.BaseScale`)))))))

(fn `PlaySound`
  (bind (_returnvalue_x _returnvalue_y _returnvalue_z) (`KismetMathLibrary.BreakVector` (`self.GetVelocity`)))
  (if (`NavMovementComponent.IsMovingOnGround` (`self.CharacterMovement`))
    (if (> (`KismetMathLibrary.VSize` (`self.GetVelocity`)) 0.0)
      (`GameplayStatics.PlaySound2D` "/Game/SFX/footstep.footstep" 1.0 1.0 0.0 null null)
      (set `self.played_jump` false)
      (set `self.played_fall` false))
    (elif (< _returnvalue_z -100.0)
      (if (not (`self.played_fall`))
        (`GameplayStatics.PlaySound2D` "/Game/SFX/wind_fall.wind_fall" 1.0 1.0 0.0 null null)
        (set `self.played_fall` true)
        (set `self.played_jump` false))
      (elif (not (`self.played_jump`))
        (`GameplayStatics.PlaySound2D` "/Game/SFX/wind_up.wind_up" 1.0 1.0 0.0 null null)
        (set `self.played_jump` true)
        (set `self.played_fall` false)))))

(fn `UpdateAnimation`
  (bind (_returnvalue_x _returnvalue_y _returnvalue_z) (`KismetMathLibrary.BreakVector` (`self.GetVelocity`)))
  (if (`NavMovementComponent.IsMovingOnGround` (`self.CharacterMovement`))
    (if (> (`KismetMathLibrary.VSize` (`self.GetVelocity`)) 0.0)
      (`PaperFlipbookComponent.SetFlipbook` (`self.Sprite`) "/Game/StarterContent/Sprites/Flipbooks/Run_LB.Run_LB")
      (else
        (`PaperFlipbookComponent.SetFlipbook` (`self.Sprite`) "/Game/StarterContent/Sprites/Flipbooks/LB_Idle.LB_Idle")))
    (elif (< _returnvalue_z -100.0)
      (`PaperFlipbookComponent.SetFlipbook` (`self.Sprite`) "/Game/StarterContent/Sprites/Flipbooks/LB_Fall.LB_Fall")
      (else
        (`PaperFlipbookComponent.SetFlipbook` (`self.Sprite`) "/Game/StarterContent/Sprites/Flipbooks/LB_Jump.LB_Jump")))))

(fn `UserConstructionScript`)