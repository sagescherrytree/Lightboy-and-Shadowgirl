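; DoorLB is the exit door for the LightBoy player, forming half of a two-door win condition with DoorSG.
; On BeginPlay it caches the first PlayerLB and DoorSG actors found in the level.
; LightBoy overlapping it sets IsActive and plays a ding, then calls Win if DoorSG is already active.
; The flag clears when LightBoy leaves the overlap.
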(event `self.ReceiveBeginPlay`
  (bind _outactors (`GameplayStatics.GetAllActorsOfClass` "/Game/Blueprints/PlayerLB.PlayerLB_C"))
  (set `self.LightBoy` (`|GetArrayItem` _outactors))
  (bind _outactors_2 (`GameplayStatics.GetAllActorsOfClass` "/Game/Blueprints/DoorSG.DoorSG_C"))
  (set `self.DoorSG` (`|GetArrayItem` _outactors_2)))

(event `self.ReceiveActorBeginOverlap`
  (params (OtherActor :type "Actor Object Reference"))
  (if (== OtherActor (`self.LightBoy`))
    (set `self.IsActive` true)
    (`GameplayStatics.PlaySound2D` "/Game/SFX/ding.ding" 1.0 1.0 0.0 null null)
    (if (`/Game/Blueprints/DoorSG.IsActive` (`self.DoorSG`))
      (`/Game/Blueprints/Lib.Win`))))

(event `self.ReceiveActorEndOverlap`
  (params (OtherActor :type "Actor Object Reference"))
  (if (== OtherActor (`self.LightBoy`))
    (set `self.IsActive` false)))

(fn `UserConstructionScript`)