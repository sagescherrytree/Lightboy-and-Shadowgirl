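; LightProbe counts how many lights reach the location of its owning actor.
; CountLights gathers every actor implementing LightInterface, asks each whether it reaches that location through Reaches, and returns the tally in NumLights.
; It runs only when called, as the BeginPlay and Tick events are disabled stubs.
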(fn `CountLights`
  (returns (NewParam :type Integer))
  (locals (_NumLights :type Integer))
  (bind _outactors (`GameplayStatics.GetAllActorsWithInterface` "/Game/Blueprints/Lights/LightInterface.LightInterface_C"))
  (for _array_element _outactors
    (bind _aslight_interface (cast `/Game/Blueprints/Lights/LightInterface` _array_element))
    (bind _reached (`/Game/Blueprints/Lights/LightInterface.Reaches` _aslight_interface (`Actor.K2_GetActorLocation` (`self.GetOwner`))))
    (if _reached
      (`/Engine/EditorBlueprintResources/StandardMacros.IncrementInt` (`local._NumLights`))))
  (return (`local._NumLights`)))