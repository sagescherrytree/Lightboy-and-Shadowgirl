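; Base light Blueprint with a procedural mesh that TurnOn, TurnOff and Flip show or hide while tracking IsOn.
; LocalRaycast takes points in actor-local space, line traces in world space and returns the hit, or the trace end on a miss, back in local space.
; It also exposes Intensity and a stub IsReachable that always returns false, and its construction script is empty.
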(fn `Flip`
  (if (`self.isOn`)
    (`self.TurnOff`)
    (else
      (`self.TurnOn`))))

(fn `getIntensity`
  (returns (Intensity :type Integer))
  (return (`self.Intensity`)))

(fn `isReachable`
  (params (xz :type "Vector2D Structure"))
  (returns (isReachable :type Boolean))
  (return false))

(fn `LocalRaycast`
  (params (Start :type "Vector Structure") (End :type "Vector Structure"))
  (returns (HitLocation :type "Vector Structure"))
  (bind _returnvalue (`KismetMathLibrary.Conv_TransformToMatrix` (`self.GetTransform`)))
  (bind (_outhit _returnvalue_2) (`KismetSystemLibrary.LineTraceSingle` (`KismetMathLibrary.Conv_Vector4ToVector` (`KismetMathLibrary.Matrix_TransformPosition` _returnvalue Start)) (`KismetMathLibrary.Conv_Vector4ToVector` (`KismetMathLibrary.Matrix_TransformPosition` _returnvalue End)) "TraceTypeQuery3"))
  (bind (_bblockinghit _binitialoverlap _time _distance _location _impactpoint _normal _impactnormal _physmat _hitactor _hitcomponent _hitbonename _bonename _hititem _elementindex _faceindex _tracestart _traceend) (`GameplayStatics.BreakHitResult` _outhit))
  (return (`KismetMathLibrary.Matrix_InverseTransformPosition` (`KismetMathLibrary.Conv_TransformToMatrix` (`self.GetTransform`)) (`KismetMathLibrary.SelectVector` _location _traceend _returnvalue_2))))

(fn `TurnOff`
  (`SceneComponent.SetHiddenInGame` (`self.ProceduralMesh`) true false)
  (set `self.isOn` false))

(fn `TurnOn`
  (`SceneComponent.SetHiddenInGame` (`self.ProceduralMesh`) false false)
  (set `self.isOn` true))

(fn `UserConstructionScript`)