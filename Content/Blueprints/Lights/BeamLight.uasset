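; Beam-shaped 2D light, a child light actor that casts a band of parallel rays in the XZ plane.
; Every tick it raycasts across BeamWidth to shape a procedural mesh strip that ends at the ray hits.
; The first tick also creates the mesh with collision and draws its triangles once into a render target.
; IsReachable reports whether a point is lit, using beam bounds and a trace back to the emitter line.
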(event `self.ReceiveBeginPlay`
  (bind _beamwidth (`self.BeamWidth`))
  (`parent.ReceiveBeginPlay`)
  (set `self.DeltaWidth` (/ _beamwidth (- (`self.NumRays`) 1)))
  (set `self.HalfBeamWidth` (/ _beamwidth 2.0)))

(event `self.ReceiveTick`
  (params (DeltaSeconds :type "Float (single-precision)"))
  (bind _proceduralmesh (`self.ProceduralMesh`))
  (`parent.ReceiveTick` DeltaSeconds)
  (bind (_vertices _uvs) (`self.GenVertices`))
  (if (`self.MeshCreated`)
    (`ProceduralMeshComponent.UpdateMeshSection_LinearColor` :`self` _proceduralmesh :`Vertices` _vertices :`UV0` _uvs)
    (else
      (bind _lightmaptriangles (`self.GenLightMapTriangles` _vertices (make `Color` 255 255 255 128)))
      (bind _triangles (`self.GenTriangles`))
      (`ProceduralMeshComponent.CreateMeshSection_LinearColor` :`self` _proceduralmesh :`Vertices` _vertices :`Triangles` _triangles :`UV0` _uvs :`bCreateCollision` true)
      (`PrimitiveComponent.SetMaterial` _proceduralmesh 0 "/Game/Materials/M_2DLight_Inst.M_2DLight_Inst")
      (set `self.MeshCreated` true)
      (bind (_canvas _size _context) (`KismetRenderingLibrary.BeginDrawCanvasToRenderTarget` "/Game/Textures/lightfnmap.lightfnmap"))
      (`Canvas.K2_DrawTriangle` _canvas null _lightmaptriangles)
      (`KismetRenderingLibrary.EndDrawCanvasToRenderTarget` _context))))

(fn `GenLightMapTriangles`
  (params (Vertices :type "Array of Vector Structure") (LightColor :type "Color Structure"))
  (returns (LightMapTriangles :type "Array of CanvasUVTri Structure"))
  (locals (_LightMapTriangles :type "Array of CanvasUVTri Structure") (Vertices :type "Array of Vector Structure"))
  (bind __lightmaptriangles (`local._LightMapTriangles`))
  (bind _lightcolor (`local.LightColor`))
  (bind _vertices (`local.Vertices`))
  (for _index (range (+ (- (`self.NumRays`) 2) 1))
    (bind _returnvalue (* _index 2))
    (bind _returnvalue_2 (`KismetMathLibrary.Conv_VectorToVector2D` (`|GetArrayItem` _vertices (+ _returnvalue 1))))
    (bind _returnvalue_3 (`KismetMathLibrary.Conv_VectorToVector2D` (`|GetArrayItem` _vertices (+ _returnvalue 2))))
    (`KismetArrayLibrary.Array_Append` __lightmaptriangles (`|MakeArray` (make `CanvasUVTri` (`KismetMathLibrary.Conv_VectorToVector2D` (`|GetArrayItem` _vertices _returnvalue)) (0.0 0.0) (`KismetMathLibrary.Conv_ColorToLinearColor` _lightcolor) _returnvalue_2 (0.0 0.0) (`KismetMathLibrary.Conv_ColorToLinearColor` _lightcolor) _returnvalue_3 (0.0 0.0) (`KismetMathLibrary.Conv_ColorToLinearColor` _lightcolor)) (make `CanvasUVTri` (`KismetMathLibrary.Conv_VectorToVector2D` (`|GetArrayItem` _vertices (+ _returnvalue 3))) (0.0 0.0) (`KismetMathLibrary.Conv_ColorToLinearColor` _lightcolor) _returnvalue_2 (0.0 0.0) (`KismetMathLibrary.Conv_ColorToLinearColor` _lightcolor) _returnvalue_3 (0.0 0.0) (`KismetMathLibrary.Conv_ColorToLinearColor` _lightcolor)))))
  (return __lightmaptriangles))

(fn `GenTriangles`
  (returns (Triangles :type "Array of Integer"))
  (locals (_Triangles :type "Array of Integer"))
  (bind __triangles (`local._Triangles`))
  (for _index (range (+ (- (`self.NumRays`) 2) 1))
    (bind _returnvalue (* _index 2))
    (bind _returnvalue_2 (+ _returnvalue 1))
    (bind _returnvalue_3 (+ _returnvalue 2))
    (`KismetArrayLibrary.Array_Append` __triangles (`|MakeArray` _returnvalue _returnvalue_2 _returnvalue_3 _returnvalue_2 (+ _returnvalue 3) _returnvalue_3)))
  (return __triangles))

(fn `GenVertices`
  (returns (Vertices :type "Array of Vector Structure") (UVs :type "Array of Vector2D Structure"))
  (locals (_Vertices :type "Array of Vector Structure") (_UVs :type "Array of Vector2D Structure"))
  (bind _returnvalue (- (`self.NumRays`) 1))
  (for _index (range (+ _returnvalue 1))
    (bind _returnvalue_2 (`KismetMathLibrary.MakeVector` 0.0 0.0 (- (* _index (`self.DeltaWidth`)) (`self.HalfBeamWidth`))))
    (`KismetArrayLibrary.Array_Add` (`local._Vertices`) _returnvalue_2)
    (bind _returnvalue_3 (/ (`KismetMathLibrary.Conv_IntToDouble` _index) (`KismetMathLibrary.Conv_IntToDouble` _returnvalue)))
    (`KismetArrayLibrary.Array_Add` (`local._UVs`) (`KismetMathLibrary.MakeVector2D` _returnvalue_3))
    (bind _hitlocation (`self.LocalRaycast` _returnvalue_2 (+ _returnvalue_2 (* (`self.RayLength`) (`KismetMathLibrary.Vector_Forward`)))))
    (`KismetArrayLibrary.Array_Add` (`local._Vertices`) _hitlocation)
    (`KismetArrayLibrary.Array_Add` (`local._UVs`) (`KismetMathLibrary.MakeVector2D` _returnvalue_3 1.0)))
  (return (`local._Vertices`) (`local._UVs`)))

(fn `isReachable`
  (params (xz :type "Vector2D Structure"))
  (returns (isReachable :type Boolean))
  (bind (_returnvalue_x _returnvalue_y) (`KismetMathLibrary.BreakVector` (`self.K2_GetActorLocation`)))
  (bind _returnvalue (`KismetMathLibrary.MakeVector` xz_X _returnvalue_y xz_Y))
  (bind _returnvalue_2 (`KismetMathLibrary.Conv_TransformToMatrix` (`self.GetTransform`)))
  (bind (_returnvalue_x_2 _returnvalue_y_2 _returnvalue_z) (`KismetMathLibrary.BreakVector` (`KismetMathLibrary.Matrix_InverseTransformPosition` _returnvalue_2 _returnvalue)))
  (if (`self.isOn`)
    (if (or (< _returnvalue_x_2 0.0) (> (`KismetMathLibrary.Abs` _returnvalue_z) (`self.HalfBeamWidth`)))
      _
      (else
        (bind (_outhit _returnvalue_3) (`KismetSystemLibrary.LineTraceSingle` _returnvalue (`KismetMathLibrary.Conv_Vector4ToVector` (`KismetMathLibrary.Matrix_TransformPosition` _returnvalue_2 (`KismetMathLibrary.MakeVector` 0.0 _returnvalue_y_2 _returnvalue_z))) "TraceTypeQuery3"))
        (return (not _returnvalue_3)))))
  (return false))

(fn `UserConstructionScript`
  (`parent.UserConstructionScript`))