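; DoorSG is a goal door for the Shadow Girl player that forms half of a paired win condition with DoorLB.
; On BeginPlay it caches the first PlayerSG and DoorLB actors found in the level.
; Overlap events set IsActive while Shadow Girl touches it, and entering while DoorLB is also active calls Win.
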(event `self.ReceiveBeginPlay`
  (bind _outactors (`GameplayStatics.GetAllActorsOfClass` "/Game/Blueprints/PlayerSG.PlayerSG_C"))
  (set `self.ShadowGirl` (`|GetArrayItem` _outactors))
  (bind _outactors_2 (`GameplayStatics.GetAllActorsOfClass` "/Game/Blueprints/DoorLB.DoorLB_C"))
  (set `self.DoorLB` (`|GetArrayItem` _outactors_2)))

(event `self.ReceiveActorBeginOverlap`
  (params (OtherActor :type "Actor Object Reference"))
  (if (== OtherActor (`self.ShadowGirl`))
    (set `self.IsActive` true)
    (if (`/Game/Blueprints/DoorLB.IsActive` (`self.DoorLB`))
      (`/Game/Blueprints/Lib.Win`))))

(event `self.ReceiveActorEndOverlap`
  (params (OtherActor :type "Actor Object Reference"))
  (if (== OtherActor (`self.ShadowGirl`))
    (set `self.IsActive` false)))

(fn `UserConstructionScript`)