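; Lever actor that flips when an actor passes through it and switches its linked Targets on or off.
; When an overlap with TriggerBox ends, the sign of the leaving actor's world X velocity must match the current state for a flip to happen, so each direction sets one state.
; A flip mirrors LeverBody's pitch, inverts IsToggled and passes the new state to each target through Toggleable.
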(event `self.TriggerBox.OnComponentEndOverlap`
  (params (OverlappedComponent :type "PrimitiveComponent Object Reference") (OtherActor :type "Actor Object Reference") (OtherComp :type "PrimitiveComponent Object Reference") (OtherBodyIndex :type Integer))
  (bind _leverbody (`self.LeverBody`))
  (if (== (< (.x (`self.GetVelocity` OtherActor)) 0.0) (`self.isToggled`))
    (`SceneComponent.K2_SetRelativeRotation` _leverbody (`KismetMathLibrary.MakeRotator` (.roll (`SceneComponent.RelativeRotation` _leverbody)) (* (.pitch (`SceneComponent.RelativeRotation` _leverbody)) -1.0) (.yaw (`SceneComponent.RelativeRotation` _leverbody))) false false)
    (bind _output_get (set `self.isToggled` (not (`self.isToggled`))))
    (for _array_element (`self.Targets`)
      (bind _astoggleable (cast `/Game/Blueprints/Toggleable` _array_element))
      (`/Game/Blueprints/Toggleable.Toggle` _astoggleable _output_get))))

(fn `UserConstructionScript`)