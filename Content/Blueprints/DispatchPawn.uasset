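; DispatchPawn is a possessed pawn that routes one player's input to two characters, LightBoy (PlayerLB) and ShadowGirl (PlayerSG).
; On BeginPlay it adds the IMC_Movement Enhanced Input context and caches the first instance of each character found in the level.
; Separate move and jump actions for each character are forwarded to that character's Move, Jump and StopJumping, so one controller drives both simultaneously.
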(event `self.ReceiveBeginPlay`
  (bind _asplayer_controller (cast `PlayerController` (`self.GetController`)))
  (`EnhancedInputSubsystemInterface.AddMappingContext` (pcsubsystem `EnhancedInputLocalPlayerSubsystem` _asplayer_controller) "/Game/Input/IMC_Movement.IMC_Movement" 1 (struct))
  (bind _outactors (`GameplayStatics.GetAllActorsOfClass` "/Game/Blueprints/PlayerLB.PlayerLB_C"))
  (set `self.LightBoy` (`|GetArrayItem` _outactors))
  (bind _outactors_2 (`GameplayStatics.GetAllActorsOfClass` "/Game/Blueprints/PlayerSG.PlayerSG_C"))
  (set `self.ShadowGirl` (`|GetArrayItem` _outactors_2)))

(event `EnhancedInput|/Game/Input/IA_Jump_LB`
  (params (ActionValue :type Boolean) (ElapsedSeconds :type "Float (double-precision)") (TriggeredSeconds :type "Float (double-precision)") (InputAction :type "InputAction Object Reference" :default "/Game/Input/IA_Jump_LB.IA_Jump_LB"))
  (bind _lightboy (`self.LightBoy`))
  (:`Started`
    (`Character.Jump` _lightboy))
  (:`Completed`
    (`Character.StopJumping` _lightboy)))

(event `EnhancedInput|/Game/Input/IA_Move_LB`
  (params (ActionValue :type "Float (double-precision)") (ElapsedSeconds :type "Float (double-precision)") (TriggeredSeconds :type "Float (double-precision)") (InputAction :type "InputAction Object Reference" :default "/Game/Input/IA_Move_LB.IA_Move_LB"))
  (:`Triggered`
    (`/Game/Blueprints/PlayerLB.Move` (`self.LightBoy`) ActionValue)))

(event `EnhancedInput|/Game/Input/IA_Jump_SG`
  (params (ActionValue :type Boolean) (ElapsedSeconds :type "Float (double-precision)") (TriggeredSeconds :type "Float (double-precision)") (InputAction :type "InputAction Object Reference" :default "/Game/Input/IA_Jump_SG.IA_Jump_SG"))
  (bind _shadowgirl (`self.ShadowGirl`))
  (:`Started`
    (`Character.Jump` _shadowgirl))
  (:`Completed`
    (`Character.StopJumping` _shadowgirl)))

(event `EnhancedInput|/Game/Input/IA_Move_SG`
  (params (ActionValue :type "Float (double-precision)") (ElapsedSeconds :type "Float (double-precision)") (TriggeredSeconds :type "Float (double-precision)") (InputAction :type "InputAction Object Reference" :default "/Game/Input/IA_Move_SG.IA_Move_SG"))
  (:`Triggered`
    (`/Game/Blueprints/PlayerSG.Move` (`self.ShadowGirl`) ActionValue)))

(fn `UserConstructionScript`)