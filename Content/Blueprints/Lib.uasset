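; Blueprint function library that handles the game's end states by showing Win or Loss screens.
; Win and Lose each call a shared Menu function, then create their widget and add it to the viewport.
; Menu pauses the game, switches the player controller to UI-only input and shows the mouse cursor.
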(fn `Lose`
  (`self.Menu` null)
  (bind _returnvalue (`|CreateWidget` "/Game/loss.loss_C"))
  (`UserWidget.AddToViewport` _returnvalue 0))

(fn `Menu`
  (bind _returnvalue (`GameplayStatics.GetPlayerController` null))
  (`GameplayStatics.SetGamePaused` null true)
  (`WidgetBlueprintLibrary.SetInputMode_UIOnlyEx` _returnvalue null)
  (set `PlayerController.bShowMouseCursor` true _returnvalue))

(fn `Win`
  (`self.Menu` null)
  (bind _returnvalue (`|CreateWidget` "/Game/win.win_C"))
  (`UserWidget.AddToViewport` _returnvalue 0))