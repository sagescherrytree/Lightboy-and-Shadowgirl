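; Player character Shadowgirl for a 2D side-view game, who loses when exposed to too much light.
; BeginPlay caches all LightInterface actors, and each Tick sums intensity from those reaching her XZ position, calling Lose above a threshold.
; A LightProbe overlap with multiple BaseLight actors also calls Lose.
; Tick picks idle, run, jump or fall flipbooks from movement state, while Move drives X-axis input and scales the sprite to face the input direction.
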(event `self.ReceiveBeginPlay`
  (set `self.BaseScale` (`SceneComponent.RelativeScale3D` (`self.Sprite`)))
  (bind _outactors (`GameplayStatics.GetAllActorsWithInterface` "/Game/Blueprints/Lights/LightInterface.LightInterface_C"))
  (for _array_element _outactors
    (bind _aslight_interface (cast `/Game/Blueprints/Lights/LightInterface` _array_element))
    (`KismetArrayLibrary.Array_Add` (`self.Lights`) _aslight_interface)))

(event `self.ReceiveTick`
  (params (DeltaSeconds :type "Float (single-precision)"))
  (`self.UpdateAnimation`)
  (`self.LightCheck`))

(event `self.LightProbe.OnComponentBeginOverlap`
  (params (OverlappedComponent :type "PrimitiveComponent Object Reference") (OtherActor :type "Actor Object Reference") (OtherComp :type "PrimitiveComponent Object Reference") (OtherBodyIndex :type Integer) (bFromSweep :type Boolean) (SweepResult :type "HitResult Structure (by ref)"))
  (if (> (`KismetArrayLibrary.Array_Length` (`PrimitiveComponent.GetOverlappingActors` OverlappedComponent "/Game/Blueprints/Lights/BaseLight.BaseLight_C")) 1)
    (`KismetSystemLibrary.PrintString` "Shadowgirl Dies :(")
    (`/Game/Blueprints/Lib.Lose`)))

(fn `LightCheck`
  (locals (Intensity :type Integer))
  (for _array_element (`self.Lights`)
    (bind _isreachable (`/Game/Blueprints/Lights/LightInterface.isReachable` _array_element (`KismetMathLibrary.MakeVector2D` (.x (`self.K2_GetActorLocation`)) (.z (`self.K2_GetActorLocation`)))))
    (if _isreachable
      (bind _intensity (`/Game/Blueprints/Lights/LightInterface.getIntensity` _array_element))
      (bind _output_get (set `local.Intensity` (+ (`local.Intensity`) _intensity 0)))
      (if (> _output_get 1)
        (`KismetSystemLibrary.PrintString` "Shadowgirl Dies :(")
        (`/Game/Blueprints/Lib.Lose`)))))

(fn `Move`
  (params (NewParam :type "Float (double-precision)"))
  (`self.AddMovementInput` (1.0 0.0 0.0) NewParam)
  (bind _result (`/Engine/EditorBlueprintResources/StandardMacros.NegateFloat` (* (.x (`self.BaseScale`)) NewParam))
    (:`  `
      (`SceneComponent.SetRelativeScale3D` (`self.Sprite`) (`KismetMathLibrary.MakeVector` _result (.y (`self.BaseScale`)) (.z (`self.BaseScale`)))))))

(fn `UpdateAnimation`
  (bind (_returnvalue_x _returnvalue_y _returnvalue_z) (`KismetMathLibrary.BreakVector` (`self.GetVelocity`)))
  (if (`NavMovementComponent.IsMovingOnGround` (`self.CharacterMovement`))
    (if (> (`KismetMathLibrary.VSize` (`self.GetVelocity`)) 0.0)
      (`PaperFlipbookComponent.SetFlipbook` (`self.Sprite`) "/Game/StarterContent/Sprites/Flipbooks/Run_SG.Run_SG")
      (else
        (`PaperFlipbookComponent.SetFlipbook` (`self.Sprite`) "/Game/StarterContent/Sprites/Flipbooks/SG_Idle.SG_Idle")))
    (elif (< _returnvalue_z -100.0)
      (`PaperFlipbookComponent.SetFlipbook` (`self.Sprite`) "/Game/StarterContent/Sprites/Flipbooks/SG_Fall.SG_Fall")
      (else
        (`PaperFlipbookComponent.SetFlipbook` (`self.Sprite`) "/Game/StarterContent/Sprites/Flipbooks/SG_Jump.SG_Jump")))))

(fn `UserConstructionScript`)