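; Movable is a toggle-driven actor that slides between its starting location and an EndPos location.
; It records its location at BeginPlay, and ToggleCounter on and off events set the movement direction forward or backward.
; Each Tick advances a clamped alpha by Speed and direction, then lerps the actor's position without sweeping, so a toggle mid-move reverses from the current point.
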(event `self.ReceiveBeginPlay`
  (set `self.StartPos` (`self.K2_GetActorLocation`)))

(event `self.ReceiveTick`
  (params (DeltaSeconds :type "Float (single-precision)"))
  (bind _output_get (set `self.LerpAlpha` (`KismetMathLibrary.FClamp` (+ (* (* DeltaSeconds (`self.Speed`)) (`self.MoveDirection`)) (`self.LerpAlpha`)))))
  (`self.K2_SetActorLocation` (`KismetMathLibrary.VLerp` (`self.StartPos`) (`self.EndPos`) _output_get)))

(event `self.ToggleCounter.ToggleOn`
  (set `self.MoveDirection` 1.0))

(event `self.ToggleCounter.ToggleOff`
  (set `self.MoveDirection` -1.0))

(fn `UserConstructionScript`)