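; PeriodicMovable is a toggle-driven actor that moves back and forth between its starting location and EndPos.
; ToggleCounter on and off events set MoveDirection to one or zero, resuming or pausing the motion.
; Tick accumulates LerpAlpha by Speed and folds it into a triangle wave with modulo and Abs, where an alpha of zero maps to EndPos.
; Movement applies the interpolated location without sweeping.
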(event `self.ReceiveBeginPlay`
  (set `self.StartPos` (`self.K2_GetActorLocation`)))

(event `self.ReceiveTick`
  (params (DeltaSeconds :type "Float (single-precision)"))
  (bind _output_get (set `self.LerpAlpha` (+ (* (* DeltaSeconds (`self.Speed`)) (`self.MoveDirection`)) (`self.LerpAlpha`))))
  (`self.K2_SetActorLocation` (`KismetMathLibrary.VLerp` (`self.StartPos`) (`self.EndPos`) (`KismetMathLibrary.Abs` (- (mod _output_get 2.0) 1.0)))))

(event `self.ToggleCounter.ToggleOn`
  (set `self.MoveDirection` 1.0))

(event `self.ToggleCounter.ToggleOff`
  (set `self.MoveDirection` 0.0))

(fn `UserConstructionScript`)