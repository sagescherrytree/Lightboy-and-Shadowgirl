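; ToggleCounter is a Blueprint toggle that counts active inputs to decide when it switches on or off.
; Increment calls ToggleOn when the count leaves zero, then raises NumActiveInputs.
; Decrement lowers the count and calls ToggleOff when it reaches zero, so overlapping inputs keep the toggle on until the last one releases.
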(fn `Decrement`
  (bind _numactiveinputs (`self.NumActiveInputs`))
  (`/Engine/EditorBlueprintResources/StandardMacros.DecrementInt` _numactiveinputs
    (:`  `
      (if (== _numactiveinputs 0)
        (`self.ToggleOff`)))))

(fn `Increment`
  (bind _numactiveinputs (`self.NumActiveInputs`))
  (if (== _numactiveinputs 0)
    (`self.ToggleOn`))
  (`/Engine/EditorBlueprintResources/StandardMacros.IncrementInt` _numactiveinputs))