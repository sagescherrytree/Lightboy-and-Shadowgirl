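; Paper2D side-scrolling player character for Lightboy, with a short jump hold time set on BeginPlay.
; Tick runs UpdateAnimation, which branches on ground, speed and fall velocity but sets the LB_Idle flipbook in every case.
; Move adds input along world X and flips control yaw to face the travel direction.
; Any actor overlapping the capsule is destroyed, with a "Lightboy at gate." debug print.
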(event `self.ReceiveBeginPlay`
  (set `self.JumpMaxHoldTime` 0.2))

(event `self.ReceiveTick`
  (params (DeltaSeconds :type "Float (single-precision)"))
  (`self.UpdateAnimation`))

(event `self.CapsuleComponent.OnComponentBeginOverlap`
  (params (OverlappedComponent :type "PrimitiveComponent Object Reference") (OtherActor :type "Actor Object Reference") (OtherComp :type "PrimitiveComponent Object Reference") (OtherBodyIndex :type Integer) (bFromSweep :type Boolean) (SweepResult :type "HitResult Structure (by ref)"))
  (`self.K2_DestroyActor` OtherActor)
  (`KismetSystemLibrary.PrintString` "Lightboy at gate."))

(fn `Move`
  (params (Amount :type "Float (double-precision)"))
  (`self.AddMovementInput` (1.0 0.0 0.0) Amount)
  (`Controller.SetControlRotation` (`self.GetController`) (select `bool` (> Amount 0.0) :`false` (`KismetMathLibrary.MakeRotator` 0.0 0.0 180.0) :`true` (`KismetMathLibrary.MakeRotator` 0.0))))

(fn `UpdateAnimation`
  (bind (_returnvalue_x _returnvalue_y _returnvalue_z) (`KismetMathLibrary.BreakVector` (`self.GetVelocity`)))
  (if (`NavMovementComponent.IsMovingOnGround` (`self.CharacterMovement`))
    (if (> (`KismetMathLibrary.VSize` (`self.GetVelocity`)) 0.0)
      (`PaperFlipbookComponent.SetFlipbook` (`self.Sprite`) "/Game/StarterContent/Sprites/Flipbooks/LB_Idle.LB_Idle")
      (else
        (`PaperFlipbookComponent.SetFlipbook` (`self.Sprite`) "/Game/StarterContent/Sprites/Flipbooks/LB_Idle.LB_Idle")))
    (elif (< _returnvalue_z -100.0)
      (`PaperFlipbookComponent.SetFlipbook` (`self.Sprite`) "/Game/StarterContent/Sprites/Flipbooks/LB_Idle.LB_Idle")
      (else
        (`PaperFlipbookComponent.SetFlipbook` (`self.Sprite`) "/Game/StarterContent/Sprites/Flipbooks/LB_Idle.LB_Idle")))))

(fn `UserConstructionScript`)